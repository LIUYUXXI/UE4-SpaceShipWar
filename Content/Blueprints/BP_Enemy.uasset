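; BP_Enemy is an enemy ship actor that gets a randomized color scheme and a scale animation for spawning.
; Its SetColor event picks random body and wing indices, maps them to preset colors, and applies them to the ship mesh through a dynamic instance of M_Base_Ship.
; The same event then plays SpawnScaleTimeline to drive the actor's uniform scale.
; Nothing in this graph calls SetColor, and BeginPlay, overlap and Tick are empty.
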(event EventBeginPlay)

(event Collision|EventActorBeginOverlap
  (params (OtherActor :type Actor%20Object%20Reference)))

(event EventTick
  (params (DeltaSeconds :type Float%20%28single-precision%29)))

(event EventSetColor
  (Variables|Default|SetBodyColorIndex (Math|Random|RandomInteger 3))
  (Variables|Default|SetWingColorIndex (Math|Random|RandomInteger 3))
  (bind _returnvalue (Rendering|Material|CreateDynamicMaterialInstance "/Game/SpaceshipBattle/Content/SpaceshipBattle/Materials/M_Base_Ship.M_Base_Ship" "None" "None" :!class /Script/Engine.KismetMaterialLibrary))
  (Rendering|Material|SetVectorParameterValue _returnvalue "Color1" (Utilities|Select :Index (Variables|Default|GetBodyColorIndex) :Option%200 "(R=0.187997,G=0.177766,B=0.942708,A=1.000000)" :Option%201 "(R=0.619792,G=0.573295,B=0.030581,A=1.000000)" :Option%202 "(R=0.072476,G=0.885417,B=0.549123,A=1.000000)" :Option%203 "(R=0.570492,G=0.111170,B=0.713542,A=1.000000)") :!class /Script/Engine.MaterialInstanceDynamic)
  (Rendering|Material|SetVectorParameterValue _returnvalue "Color2" (Utilities|Select :Index (Variables|Default|GetWingColorIndex) :Option%200 "(R=0.703125,G=0.006746,B=0.264975,A=1.000000)" :Option%201 "(R=0.031023,G=0.640625,B=0.589580,A=1.000000)") :!class /Script/Engine.MaterialInstanceDynamic)
  (Rendering|Material|SetMaterial (Variables|Default|GetShipSM) 0 _returnvalue)
  (bind _scale (Timeline|SpawnScaleTimeline Play)
    (:Update
      (Transformation|SetActorScale3D (Math|Conversions|ToVector(Float) _scale)))))

(fn ConstructionScript)